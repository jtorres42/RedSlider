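; Enemy spawner actor that repeatedly spawns Ball actors at its own transform and registers itself with the RedCube_Character player on BeginPlay.
; A one-second looping timer counts down the Time variable, then starts a looping spawn timer with an interval picked once between FirstTime and SecondTime.
; When the player's Score exceeds 100, it swaps to a second spawn loop with its own short random interval, also picked once.
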(event `self.ReceiveBeginPlay`
  (bind _asred_cube_character (cast `/Game/Blueprints/Player/RedCube_Character` (`GameplayStatics.GetPlayerCharacter` 0)))
  (set `/Game/Blueprints/Player/RedCube_Character.SpawnRef` self _asred_cube_character)
  (bind _returnvalue (`KismetSystemLibrary.K2_SetTimerDelegate` (delegate `StartTime`) 1.0 true))
  (set `self.ClearTimer` _returnvalue))

(event `StartTime`
  (bind _time (`self.Time`))
  (set `self.Time` (- _time 1))
  (if (<= _time 0)
    (`KismetSystemLibrary.K2_ClearAndInvalidateTimerHandle` (`self.ClearTimer`))
    (bind _returnvalue (`KismetSystemLibrary.K2_SetTimerDelegate` (delegate `Play`) (`KismetMathLibrary.RandomFloatInRange` (`self.FirstTime`) (`self.SecondTime`)) true))
    (set `self.Timer2` _returnvalue)))

(event `Play`
  (`|SpawnActorFromClass` "/Game/Blueprints/Enemies/Ball.Ball_C" (`self.GetTransform`) "Undefined" "OverrideRootScale" null null)
  (bind _asred_cube_character (cast `/Game/Blueprints/Player/RedCube_Character` (`GameplayStatics.GetPlayerCharacter` 0)))
  (if (not (<= (`/Game/Blueprints/Player/RedCube_Character.Score` _asred_cube_character) 100))
    (`KismetSystemLibrary.K2_ClearAndInvalidateTimerHandle` (`self.Timer2`))
    (bind _returnvalue (`KismetSystemLibrary.K2_SetTimerDelegate` (delegate `PLSAY2`) (`KismetMathLibrary.RandomFloatInRange` 0.5 1.0) true))
    (set `self.tIME3` _returnvalue)))

(event `PLSAY2`
  (`|SpawnActorFromClass` "/Game/Blueprints/Enemies/Ball.Ball_C" (`self.GetTransform`) "Undefined" "OverrideRootScale" null null))

(fn `UserConstructionScript`)